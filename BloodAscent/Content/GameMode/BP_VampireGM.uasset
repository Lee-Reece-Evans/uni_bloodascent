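; VR game mode that runs enemy waves, gate opening and the skeleton finale, using a motion controller pawn.
; StartWave configures up to three waves, each a delayed loop spawning enemies at random registered points, with later waves alternating two types.
; IsWaveOver starts the next wave when no bots remain.
; ParticleWave recursively fires a fireball from each light at the skeleton, then replaces it with SpawnLady; EndGame loads TutorialMap.
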(event Custom|Start%20Wave
  (bind _spawnpoints (Variables|Default|GetSpawnPoints))
  (bind _returnvalue (Utilities|Array|Length _spawnpoints))
  (bind _returnvalue_2 (- _returnvalue 1))
  (bind _returnvalue_3 (Math|Random|RandomIntegerinRange 0 _returnvalue_2))
  (bind _output (Utilities|Array|Get(acopy) _spawnpoints _returnvalue_3))
  (bind _returnvalue_4 (Math|Transform|MakeTransform _output))
  ;[1 1 1] Start Wave
  (Math|Integer|IncrementInt (Variables|Default|GetWaveNum)
    (:%20%20
      (Utilities|FlowControl|Delay 4.0)
      (Variables|Default|SetTimeTillBotActivates 5.0)
      (switch int (Variables|Default|GetWaveNum)
        (:1
          (Variables|Default|SetBotDelayTime 5.0)
          (Variables|Default|SetBotsWanted 5)
          (Variables|Default|SetTotalBotsAlive (Variables|Default|GetBotsWanted))
          (Utilities|FlowControl|Delay (Variables|Default|GetBotDelayTime) :!label _label)
          (if (< (Variables|Default|GetBotsSpawned) (Variables|Default|GetBotsWanted))
            (bind _result (Math|Integer|IncrementInt (Variables|Default|GetBotsSpawned))
              (:%20%20
                (Variables|Default|SetBotsSpawned _result)
                (CallFunction|SpawnAI (Math|Transform|MakeTransform _output) "NewEnumerator0")
                (goto _label)))
            (else
              (Variables|Default|SetBotsSpawned 0))))
        (:2
          (Variables|Default|SetBotDelayTime 4.0)
          (Variables|Default|SetBotsWanted 7)
          (Variables|Default|SetTotalBotsAlive (Variables|Default|GetBotsWanted))
          (Utilities|FlowControl|Delay (Variables|Default|GetBotDelayTime) :!label _label_2)
          (if (< (Variables|Default|GetBotsSpawned) (Variables|Default|GetBotsWanted))
            (bind _result_2 (Math|Integer|IncrementInt (Variables|Default|GetBotsSpawned))
              (:%20%20
                (Variables|Default|SetBotsSpawned _result_2)
                (Utilities|FlowControl|FlipFlop
                  (:A
                    (CallFunction|SpawnAI _returnvalue_4 "NewEnumerator0")
                    (goto _label_2))
                  (:B
                    (CallFunction|SpawnAI _returnvalue_4 "NewEnumerator1")
                    (goto _label_2)))))
            (else
              (Variables|Default|SetBotsSpawned 0))))
        (:3
          (Variables|Default|SetBotDelayTime 3.5)
          (Variables|Default|SetBotsWanted 8)
          (Variables|Default|SetTotalBotsAlive (Variables|Default|GetBotsWanted))
          (goto _label_2))))))

(event Custom|EndGame
  ;[1 1 1] Endgame called by skeleton sequence event
  (Utilities|FlowControl|Delay 5.0)
  (Game|OpenLevel(byName) "TutorialMap")
  (Variables|Default|SetcanTeleport true))

(event Custom|IsWaveOver?
  ;[1 1 1] WaveOver?
  (if (== (Variables|Default|GetTotalBotsAlive) 0)
    (CallFunction|StartWave)))

(event Custom|SpawnAI
  (params (SpawnTransform :type Transform) (EnemyType :type EnemyTypes%20Enum :default "NewEnumerator0"))
  ;[1 1 1] Do a little dance, make a little love. get down tonight
  (Game|SpawnActorfromClass "/Game/VirtualRealityBP/Blueprints/Enemy_BP.Enemy_BP_C" SpawnTransform "AdjustIfPossibleButAlwaysSpawn" 0 EnemyType 0))

(event Custom|ParticleWave
  ;[1 1 1] Turn all ligjts off at once
  (Utilities|FlowControl|Delay 0.2)
  (for _array_element (Variables|Default|GetLights)
    (Default|TurnOffLight _array_element))
  (CallFunction|GoThroughEachLight))

(event Custom|GoThroughEachLight
  (bind _lights (Variables|Default|GetLights))
  (bind _lightsequence (Variables|Default|GetLightSequence))
  (bind _output (Utilities|Array|Get(acopy) _lights _lightsequence))
  (bind _returnvalue (Transformation|GetActorLocation _output))
  ;[1 1 1] Turn on Each Light
  (Utilities|FlowControl|Delay 2.0)
  (Default|TurnonLight _output)
  (Game|SpawnActorfromClass "/Game/VirtualRealityBP/Blueprints/Weapons/FireBall.FireBall_C" (Math|Transform|MakeTransform _returnvalue (Math|Rotator|FindLookatRotation _returnvalue (Transformation|GetActorLocation (Variables|Default|GetSkeleton)))) "AlwaysSpawn" 0 1.5e+03 0)
  (Utilities|FlowControl|Delay 1.0)
  (Default|TurnOffLight _output)
  (Math|Integer|IncrementInt (Variables|Default|GetLightSequence)
    (:%20%20
      (if (< (Variables|Default|GetLightSequence) (Utilities|Array|Length (Variables|Default|GetLights)))
        (CallFunction|GoThroughEachLight)
        (else
          (for _array_element (Variables|Default|GetLights)
            (Default|TurnonLight _array_element))
          ;;[1 1 1] Spawn lady and end game
          (Game|SpawnActorfromClass "/Game/VirtualRealityBP/Blueprints/SpawnLady.SpawnLady_C" (Math|Transform|MakeTransform (Transformation|GetActorLocation (Variables|Default|GetSkeleton))) "AlwaysSpawn" 0 0)
          (Actor|DestroyActor (Variables|Default|GetSkeleton)))))))

(event Custom|OpenGates
  ;[1 1 1] open gates
  (for _array_element (Variables|Default|GetGates)
    (bind _asgate (Utilities|Casting|CastToGate _array_element))
    (Default|ActivateGate _asgate)))

(event Custom|SetSpawnPoints
  (params (Spawn :type Vector))
  (Utilities|Array|Add (Variables|Default|GetSpawnPoints) Spawn))

(event EventBeginPlay
  ;[1 1 1] BeginPlay
  (bind _outactors (Actor|GetAllActorsOfClass "/Game/VirtualRealityBP/Blueprints/Gate.Gate_C"))
  (Variables|Default|SetGates _outactors))

(fn ConstructionScript
  (Variables|Default|SetDefaultPawnClass "/Game/VirtualRealityBP/Blueprints/MotionControllerPawn.MotionControllerPawn_C"))